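; BP_BaseAI is an exploding enemy that chases a random living player at a randomized walk speed.
; The server re-issues the move every second, picking another target if the current pawn becomes invalid.
; Player overlap triggers a multicast explosion and sphere-trace GameplayEffect damage, then death.
; Damage briefly shows a health bar; lethal damage drops health or energy pickups, and death hides the AI and removes it from its spawner.
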(event `self.ReceiveBeginPlay`
  ;[1 1 1] When spawned into the world we first ensure we dont collide and deal damage, wait for half a sec, choose a random walk speed and random active player, then chase them
  (`self.EnsureWidgetRefIsSet`)
  (`/Engine/EditorBlueprintResources/ActorMacros.Switch Has Authority`
    (:`Authority`
      (`KismetSystemLibrary.Delay` 0.5)
      (set `CharacterMovementComponent.MaxWalkSpeed` (`KismetMathLibrary.RandomFloatInRange` 250.0 650.0) (`self.CharacterMovement`))
      (`|ExecutionSequence`
        (:`then_0`
          (`self.ChooseRandomPlayerToChase`))))))

(event `Killed`
  ;[1 1 1] When the AI is killed, we remove ourselfs from the spawners array and set our life span
  (`self.MulticastAIKilled`)
  (`self.RemoveSelfFromSpawner`)
  (`self.SetLifeSpan` 1.0))

(event `EnsureWidgetRefIsSet`
  ;[1 1 1] We have to ensure we set the AI's reference in the widget otherwise we can display the health
  (bind _asw_aihealth (cast `/Game/UI/W_AIHealth` (`WidgetComponent.GetWidget` (`self.HealthWidget`))))
  (set `/Game/UI/W_AIHealth.As BP Base AI` self _asw_aihealth))

(event `MulticastExplosion`
  ;[1 1 1] Multicast events for exploading the AI and hiding the mesh
  (`ActorComponent.SetActive` (`self.Explosion`) true false)
  (if (not (`KismetSystemLibrary.IsDedicatedServer`))
    (`GameplayStatics.SpawnSoundAtLocation` "/Game/Sounds/explosion_Cue.explosion_Cue" (`SceneComponent.K2_GetComponentLocation` (`self.CapsuleComponent`)) (struct) 1.0 1.0 0.0 "/Game/Sounds/DefaultSoundATT.DefaultSoundATT" null)))

(event `MulticastAIKilled`
  ;[1 1 1] Multicast events for exploading the AI and hiding the mesh
  (`self.HideMeshAndCollision`))

(event `self.DealDamageToAI`
  (params (DamageAmount :type "Float (single-precision)"))
  ;[1 1 1] Called from the server to deal damage to the AI
  (`self.DealDamage` DamageAmount))

(event `self.DamageSphere.OnComponentBeginOverlap`
  (params (OverlappedComponent :type "PrimitiveComponent Object Reference") (OtherActor :type "Actor Object Reference") (OtherComp :type "PrimitiveComponent Object Reference") (OtherBodyIndex :type Integer) (bFromSweep :type Boolean) (SweepResult :type "HitResult Structure (by ref)"))
  ;[1 1 1] When a actor overlaps the damage sphere, we will trace out and damage any actor in the area
  (`/Engine/EditorBlueprintResources/ActorMacros.Switch Has Authority`
    (:`Authority`
      (cast `/Game/ThirdPerson/Blueprints/BP_ThirdPersonCharacter` OtherActor)
      (`Controller.StopMovement` (`AIBlueprintHelperLibrary.GetAIController` self))
      (`self.SphereTraceForDamage`))))

(event `MulticastShowHealthBar`
  ;[1 1 1] Only show the health widget when someone shoots it
  (`SceneComponent.SetVisibility` (`self.HealthWidget`) true false)
  (`KismetSystemLibrary.RetriggerableDelay` 10.0)
  (`SceneComponent.SetVisibility` (`self.HealthWidget`) false false))

(fn `DealDamage`
  (params (Damage :type "Float (double-precision)"))
  (bind _health (`self.Health`))
  ;[1 1 1] When the AIs health reaches 0, spawn a attribute drop and kill the AI
  (if (not (== _health 0.0))
    (bind _output_get (set `self.Health` (`KismetMathLibrary.FClamp` (- _health Damage) 0.0 (`self.MaxHealth`))))
    (if (== _output_get 0.0)
      (`|SpawnActorFromClass` (select `bool` (`KismetMathLibrary.RandomBoolWithWeight` 0.2) :`false` "/Game/AI/BP_EnergyDrop.BP_EnergyDrop_C" :`true` "/Game/AI/BP_HealthDrop.BP_HealthDrop_C" :!type "Actor Class Reference") (`KismetMathLibrary.MakeTransform` (`SceneComponent.K2_GetComponentLocation` (`self.CapsuleComponent`))) "AdjustIfPossibleButAlwaysSpawn" "MultiplyWithRoot" self null)
      (`self.Killed`)
      (else
        (`self.MulticastShowHealthBar`)))))

(fn `HideMeshAndCollision`
  (`SceneComponent.SetVisibility` (`self.Mesh`) false true)
  (`SceneComponent.SetVisibility` (`self.HealthWidget`) false true)
  (`PrimitiveComponent.SetCollisionEnabled` (`self.CapsuleComponent`) "NoCollision")
  (`PrimitiveComponent.SetCollisionEnabled` (`self.Mesh`) "NoCollision")
  (`PrimitiveComponent.SetCollisionEnabled` (`self.Sphere`) "NoCollision")
  (`PrimitiveComponent.SetCollisionEnabled` (`self.Cube`) "NoCollision"))

(fn `OnRep_Health`)

(fn `OnRep_MaxHealth`)

(fn `SphereTraceForDamage`
  (bind _returnvalue (`SceneComponent.K2_GetComponentLocation` (`self.DamageSphere`)))
  (`PrimitiveComponent.SetCollisionEnabled` (`self.DamageSphere`) "NoCollision")
  (`self.MulticastExplosion`)
  (bind _outhits (`KismetSystemLibrary.SphereTraceMultiForObjects` _returnvalue _returnvalue 175.0 (`|MakeArray` "ObjectTypeQuery3" :!type "EObjectTypeQuery Enum") false (`|MakeArray` self :!type "Actor Object Reference") "None" true (struct :`R` 1.0 :`A` 1.0) (struct :`G` 1.0 :`A` 1.0) 10.0))
  (for _array_element _outhits
    (bind _asbp_third_person_character (cast `/Game/ThirdPerson/Blueprints/BP_ThirdPersonCharacter` (`.HitActor` (`GameplayStatics.BreakHitResult` _array_element))))
    (`Damage.DealDamageToPlayer` _asbp_third_person_character "/Game/GAS/Effects/GE_AIDamageDeal.GE_AIDamageDeal_C"))
  (`self.Killed`))

(fn `UserConstructionScript`)