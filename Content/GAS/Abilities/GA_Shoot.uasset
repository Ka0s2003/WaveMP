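; Gameplay ability that fires the third-person character's weapon.
; On activation, the authority applies the shot energy effect to the owner, and the owning character is cached.
; An attenuated shot sound plays at the character's capsule on any non-dedicated-server instance running the ability.
; Only the locally controlled instance calls ShootWeapon on the character, then ends the ability after a short delay.
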(event `self.K2_ActivateAbility`
  ;[1 1 1] Only shoot locally and have the authority apply the effect
  (`self.K2_HasAuthority`
    (:`True`
      (`self.BP_ApplyGameplayEffectToOwner` "/Game/GAS/Effects/GE_ShotEnergy.GE_ShotEnergy_C"))
    (:`False`
      _))
  (bind _asbp_third_person_character (cast `/Game/ThirdPerson/Blueprints/BP_ThirdPersonCharacter` (`.OwnerActor` (break `GameplayAbilityActorInfo` (`self.GetActorInfo`)))))
  (set `self.OwningCharacter` _asbp_third_person_character)
  (`self.SpawnShotSound`)
  (if (`Pawn.IsLocallyControlled` _asbp_third_person_character)
    (`WaveMPCharacter.ShootWeapon` _asbp_third_person_character)
    (`KismetSystemLibrary.Delay` 0.1)
    (`self.K2_EndAbility`)))

(event `SpawnShotSound`
  ;[1 1 1] Spawn the shot sound at the characters location
  (if (not (`KismetSystemLibrary.IsDedicatedServer`))
    (bind _owningcharacter (`self.OwningCharacter`)
      (:`then`
        (`GameplayStatics.SpawnSoundAtLocation` "/Game/Sounds/Shoot_Cue.Shoot_Cue" (`SceneComponent.K2_GetComponentLocation` (`Character.CapsuleComponent` _owningcharacter)) (struct) 1.0 1.0 0.0 "/Game/Sounds/DefaultSoundATT.DefaultSoundATT" null))
      (:`else`))))