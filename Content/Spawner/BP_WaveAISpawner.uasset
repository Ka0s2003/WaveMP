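; Server-authoritative wave spawner that waits for a player to join, then runs endless, growing waves of AI with multicast round sounds.
; Delayed loops stagger spawns at random navmesh points around a fixed origin, tracking each AI in an alive array.
; A polling macro watches that array and starts the next wave once empty, updating the WaveMPGameMode between Waiting and Playing.
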(event `self.ReceiveBeginPlay`
  ;[1 1 1] Waits for atleast 1 player to join the server before starting the waves
  (`/Engine/EditorBlueprintResources/ActorMacros.Switch Has Authority`
    (:`Authority`
      (`self.GetCurrentGameMode`)
      (`self.WaitForAPlayer`
        (:`true`
          (`KismetSystemLibrary.Delay` 2.0)
          (`self.StartWave`))))))

(event `StartWave`
  ;[1 1 1] Spawns the first wave of AI, we use delayed for loops so when there are lots of actors to spawn it, they spawn in nicely
  (bind _as_wave_mpgame_mode (`self.As Wave MPGame Mode`)
    (:`then`
      (`WaveMPGameMode.StartGameTimer` _as_wave_mpgame_mode)
      (`self.MultiCastRoundSounds` false)
      (`self.DelayForLoop` 0 (`KismetMathLibrary.RandomIntegerInRange` (`self.MinStartingAI`) (`self.MaxStartingAI`)) 0.2
        (:`LoopBody`
          (`self.SpawnNewAI`))
        (:`Completed`
          (`self.MonitorCurrentWave`))))
    (:`else`)))

(event `MultiCastRoundSounds`
  (params (`Wait?` :type Boolean))
  ;[1 1 1] Tell all clients to play a sound
  (if (not (`KismetSystemLibrary.IsDedicatedServer`))
    (`GameplayStatics.PlaySound2D` (select `bool` `Wait?` :`false` "/Game/Sounds/NewWave.NewWave" :`true` "/Game/Sounds/suspense-dark.suspense-dark" :!type "SoundBase Object Reference") 0.6 1.0 0.0 null null)))

(event `NextWave`
  ;[1 1 1] Spawns additional waves of AI
  (bind _as_wave_mpgame_mode (`self.As Wave MPGame Mode`)
    (:`then`
      (`WaveMPGameMode.SetNewGameState` _as_wave_mpgame_mode "Waiting")
      (set `self.MinStartingAI` (`self.MaxStartingAI`))
      (set `self.MaxStartingAI` (`KismetMathLibrary.RandomIntegerInRange` (+ (`self.MaxStartingAI`) 1) (+ (`self.MaxStartingAI`) 3)))
      (`self.MultiCastRoundSounds` true)
      (`KismetSystemLibrary.Delay` (`self.TimeBetweenWaves`))
      (`self.MultiCastRoundSounds` false)
      (`self.DelayForLoop` 0 (`KismetMathLibrary.RandomIntegerInRange` (`self.MinStartingAI`) (`self.MaxStartingAI`)) 0.2
        (:`LoopBody`
          (`self.SpawnNewAI`))
        (:`Completed`
          (`self.MonitorCurrentWave`))))
    (:`else`)))

(fn `GetCurrentGameMode`
  (bind _returnvalue (`GameplayStatics.GetGameMode`))
  (`/Engine/EditorBlueprintResources/StandardMacros.IsValid` _returnvalue
    (:`Is Valid`
      (bind _aswave_mpgame_mode (cast `WaveMPGameMode` _returnvalue))
      (set `self.As Wave MPGame Mode` _aswave_mpgame_mode))))

(fn `RemoveSelfFromArray`
  (params (AIToRemove :type "/Game/AI/BP_BaseAI Object Reference"))
  (returns (`Removed?` :type Boolean))
  (bind _currentaialive (`self.CurrentAIAlive`))
  (if (`KismetArrayLibrary.Array_Contains` _currentaialive AIToRemove)
    (bind _returnvalue (`KismetArrayLibrary.Array_RemoveItem` _currentaialive AIToRemove)))
  (return _returnvalue))

(fn `SpawnNewAI`
  (bind (_randomlocation _returnvalue) (`NavigationSystemV1.K2_GetRandomLocationInNavigableRadius` (`KismetMathLibrary.MakeVector` 4210.0 4150.0) 9000.0 null "/Script/NavigationSystem.RecastFilter_UseDefaultArea"))
  (if _returnvalue
    (bind _returnvalue_2 (`|SpawnActorFromClass` (`self.BaseAIClass`) (`KismetMathLibrary.MakeTransform` _randomlocation) "Undefined" "MultiplyWithRoot" self self null))
    (`/Engine/EditorBlueprintResources/StandardMacros.IsValid` _returnvalue_2
      (:`Is Valid`
        (`KismetArrayLibrary.Array_Add` (`self.CurrentAIAlive`) _returnvalue_2)))))

(fn `UserConstructionScript`)