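; Base player controller that sets up the in-game HUD and handles the player's switch to spectating on death.
; On BeginPlay it sets game-only input and adds the game status widget to the viewport.
; On a death notification it triggers the death widget, records the pawn's location and flags itself dead.
; After a short delay it unpossesses, then spawns and possesses a spectator pawn at that location.
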(event `self.ReceiveBeginPlay`
  ;[1 1 1] Ensure your input mode is game only
  (`WidgetBlueprintLibrary.SetInputMode_GameOnly` self true)
  (`self.CreateGameStateWidget`))

(event `self.NotifyPlayerDead`
  ;[1 1 1] When dead, show the death widget, get the location where you died and set dead to true, unpossess your current character and spawn a spectator
  (`self.ShowClientDeath`)
  (set `self.SpectatorLocation` (`self.K2_GetActorLocation` (`self.K2_GetPawn`)))
  (`self.SetDead` true)
  (`KismetSystemLibrary.Delay` 3.0)
  (`self.UnPossess`)
  (bind _returnvalue (`|SpawnActorFromClass` "/Script/Engine.SpectatorPawn" (`KismetMathLibrary.MakeTransform` (`self.SpectatorLocation`)) "AdjustIfPossibleButAlwaysSpawn" "MultiplyWithRoot" self null))
  (`self.Possess` _returnvalue))

(event `ShowClientDeath`
  ;[1 1 1] Displays Death widget
  (`self.DisplayDeathWidget`))

(event `CreateGameStateWidget`
  ;[1 1 1] Adds the game status widget
  (bind _returnvalue (`|CreateWidget` "/Game/UI/W_GameStatus.W_GameStatus_C" self))
  (`/Engine/EditorBlueprintResources/StandardMacros.IsValid` _returnvalue
    (:`Is Valid`
      (`UserWidget.AddToViewport` _returnvalue 1))))

(fn `UserConstructionScript`)